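; Coin is a collectible pickup that adds to the first-person player's coin count when touched.
; On overlap with an actor tagged Player, it casts to BP_FirstPersonCharacter and increments that character's CoinsCollected.
; It then prints the new total as a debug string and destroys itself.
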(event Collision|EventActorBeginOverlap
  (params (OtherActor :type Actor%20Object%20Reference))
  (if (Actor|ActorHasTag OtherActor "Player")
    (bind _asbp_first_person_character (Utilities|Casting|CastToBP_FirstPersonCharacter OtherActor))
    (bind _result (Math|Integer|IncrementInt (Variables|/Game/FirstPerson/Blueprints/BP_FirstPersonCharacter.BP_FirstPersonCharacter_C|GetCoins%20Collected _asbp_first_person_character))
      (:%20%20
        (bind _output_get (Variables|/Game/FirstPerson/Blueprints/BP_FirstPersonCharacter.BP_FirstPersonCharacter_C|SetCoins%20Collected _asbp_first_person_character _result))
        (bind _output_get_2 (Variables|Default|SetCoins%20Amount%20String "Coins Collected: "))
        (Development|PrintString (Utilities|String|Append _output_get_2 (Utilities|String|ToString(Integer) _output_get)))
        (Actor|DestroyActor)))))

(fn ConstructionScript)