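; Fire hazard actor that sets overlapping entities on fire while they remain inside it.
; On begin overlap, it looks up the other actor's EntityController component and calls SetOnFire with its Damage and DamageInterval values.
; On end overlap, it calls the same function to clear the fire state and zero both values, leaving the burn handling to that component.
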(event Collision|EventActorBeginOverlap
  (params (OtherActor :type Actor%20Object%20Reference))
  (bind _returnvalue (Actor|GetComponentbyClass OtherActor "/Script/UE5Level.EntityController"))
  (if (Utilities|IsValid _returnvalue)
    (Class|EntityController|SetonFire _returnvalue true (Variables|Default|GetDamage) (Variables|Default|GetDamage%20Interval))))

(event Collision|EventActorEndOverlap
  (params (OtherActor :type Actor%20Object%20Reference))
  (bind _returnvalue (Actor|GetComponentbyClass OtherActor "/Script/UE5Level.EntityController"))
  (if (Utilities|IsValid _returnvalue)
    (Class|EntityController|SetonFire _returnvalue false 0.0 0.0)))

(fn ConstructionScript)