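; Molotov Blueprint that starts a fire where it hits the ground.
; Its HitGround event spawns a Fire actor slightly above the stored HitPosition.
; It has no other active logic: the default events are disabled and the construction script only calls its parent.
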(event EventBeginPlay
  (|CallParentFunction) ; This node is disabled and will not be called.\nDrag off pins to build functionality.
)

(event Collision|EventActorBeginOverlap
  (params (OtherActor :type Actor%20Object%20Reference))
  (|CallParentFunction OtherActor) ; This node is disabled and will not be called.\nDrag off pins to build functionality.
)

(event EventTick
  (params (DeltaSeconds :type Float%20%28single-precision%29))
  (|CallParentFunction DeltaSeconds) ; This node is disabled and will not be called.\nDrag off pins to build functionality.
)

(event EventHitGround
  (Game|SpawnActorfromClass "/Game/Blueprints/Fire.Fire_C" (Math|Transform|MakeTransform (+ (Variables|Default|GetHit%20Position) "0.000000,0.000000,50.000000") "0, 0, 0" "1.000000,1.000000,1.000000") "Undefined" "MultiplyWithRoot" 0 0))

(fn ConstructionScript
  (|CallParentFunction))